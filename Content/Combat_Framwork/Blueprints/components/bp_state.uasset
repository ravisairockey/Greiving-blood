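; State component in the combat framework that holds the owner's current gameplay tag state and a movement input flag.
; Functions set or clear the state, or test it against a tag container using non-exact, hierarchical matching.
; A movement input event either disables the flag immediately, or waits on a retriggerable delay, then re-enables it and clears the state.
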(event `movement input handler`
  (params (Duration :type "Float (double-precision)") (`Disable Input` :type Boolean))
  (if `Disable Input`
    (set `self.MovementInput` false)
    (else
      (`KismetSystemLibrary.RetriggerableDelay` Duration)
      (set `self.MovementInput` true)
      (`self.ClearState`))))

(fn `ClearState`
  (set `self.CurrentState` (struct)))

(fn `IsCurrentStateEqualToAny`
  (params (`State To Check` :type "GameplayTagContainer Structure"))
  (returns (ReturnValue :type Boolean))
  (return (`BlueprintGameplayTagLibrary.HasTag` `State To Check` (`self.CurrentState`))))

(fn `SetState`
  (params (NewState :type "GameplayTag Structure"))
  (set `self.CurrentState` NewState))