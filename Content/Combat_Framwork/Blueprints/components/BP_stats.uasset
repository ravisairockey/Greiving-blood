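; BP_stats is a combat framework component that tracks player stamina, with functions to check and deduct a cost.
; Each stamina change calls UpdateStats.
; Regeneration runs on a looping function-name timer that adds the regen rate until stamina reaches its maximum.
; A Handle Stamina Regen graph starts that timer through a gate after a delay, or stops it and closes the gate to block a pending restart.
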(event `RefreshStamina`
  (params (StartStaminaRegen :type Boolean))
  (if StartStaminaRegen
    (`KismetSystemLibrary.K2_SetTimer` null "RegenrateStamina" 0.1 true)
    (else
      (`KismetSystemLibrary.K2_ClearTimer` null "RegenrateStamina"))))

(event `Handle stamina regen event`
  (params (`Start Refresh Stamina` :type Boolean) (Duration :type "Float (double-precision)"))
  (`self.Handle Stamina Regen` `Start Refresh Stamina` Duration))

(fn `Check player has enough stamina`
  (params (`Stamina Cost` :type "Float (double-precision)"))
  (returns (ReturnValue :type Boolean))
  (return (>= (`self.BaseStamina`) `Stamina Cost`)))

(fn `Decrease Stamina`
  (params (StaminaCost :type "Float (double-precision)"))
  (set `self.BaseStamina` (- (`self.BaseStamina`) StaminaCost))
  (`self.UpdateStats`))

(fn `RegenrateStamina`
  (bind _output_get (set `self.BaseStamina` (+ (`self.BaseStamina`) (`self.StaminaRegenRate`))))
  (`self.UpdateStats`)
  (if (>= _output_get (`self.MaxStamina`))
    (`self.RefreshStamina` false)))