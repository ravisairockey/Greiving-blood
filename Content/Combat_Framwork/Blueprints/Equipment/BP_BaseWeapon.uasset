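; Base weapon Blueprint that handles equipping and supplies combo animation montages for combat actions.
; Construction applies the equipment mesh, and equipping registers the weapon with the owner's BP_Combat component, attaching it to the equipped or unequipped socket by combat state.
; Montage lookup reads a data table row named after the action enum and steps through its animation array.
; The combo index resets after the last animation or when a retriggerable delay expires.
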(event `Attack Combo counter`
  (`/Engine/EditorBlueprintResources/StandardMacros.IncrementInt` (`self.AnimationIndex`)
    (:`  `
      (`KismetSystemLibrary.RetriggerableDelay` 2.0)
      (set `self.AnimationIndex` 0 :!label _label))))

(event `Reset Animation Index`
  (goto _label))

(fn `Equip item`
  (bind _output_get (set `self.CombatComponentRef` (`self.GetComponentByClass` (`self.GetOwner`) "/Game/Combat_Framwork/Blueprints/components/BP_Combat.BP_Combat_C")))
  (`/Game/Combat_Framwork/Blueprints/components/BP_Combat.SetWeapon` _output_get self)
  (`self.Attach to Player` (select `bool` (`/Game/Combat_Framwork/Blueprints/components/BP_Combat.CombatEnabled?` (`self.CombatComponentRef`)) :`false` (`self.UnequipedSocket`) :`true` (`self.EquipedSocket`))))

(fn `Get Montage For Action`
  (params (Action :type "/Game/Combat_Framwork/Blueprints/Enums/E_MontageAction Enum" :default "NewEnumerator0"))
  (returns (Output :type "AnimMontage Object Reference"))
  (bind _returnvalue (`|GetDataTableRow` (`self.Animationdatatable`) (`KismetStringLibrary.Conv_StringToName` (`|GetEnumeratorNameAsString` Action)))
    (:`then`
      (bind ((`Animation_6_26472AD94EBFC0AF7ED664B009D8F73E` _animation)) (break `/Game/Combat_Framwork/Blueprints/Structs/S_MontageAction` _returnvalue))
      (if (>= (`self.AnimationIndex`) (- (`KismetArrayLibrary.Array_Length` _animation) 1))
        (`self.Reset Animation Index`)
        (return (`|GetArrayItem` _animation (`KismetArrayLibrary.Array_LastIndex` _animation)))
        (else
          (`self.Attack Combo counter`)
          (return (`|GetArrayItem` _animation (- (`self.AnimationIndex`) 1))))))))

(fn `UserConstructionScript`
  (`StaticMeshComponent.SetStaticMesh` (`self.StaticMesh`) (`self.EquipmentMesh`)))